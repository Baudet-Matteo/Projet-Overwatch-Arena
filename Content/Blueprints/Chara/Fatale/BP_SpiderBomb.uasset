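; BP_SpiderBomb is a bomb actor that sticks to the surface beneath it and later removes itself.
; Each tick, a short Visibility trace runs along the mesh's local down axis.
; On a hit, the mesh snaps to the point, aligns to the normal, stops physics and gravity, then destroys itself after a delay.
; A longer BeginPlay timeout also destroys it; no explosion or damage logic is present.
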(event `self.ReceiveBeginPlay`
  (`KismetSystemLibrary.Delay` 20.0)
  (`self.K2_DestroyActor`))

(event `self.ReceiveTick`
  (params (DeltaSeconds :type "Float (single-precision)"))
  (bind _staticmesh (`self.StaticMesh`))
  (bind _staticmesh_2 (`self.StaticMesh`))
  (bind _returnvalue (`SceneComponent.K2_GetComponentLocation` _staticmesh_2))
  (bind (_outhit _returnvalue_2) (`KismetSystemLibrary.LineTraceSingle` _returnvalue (+ _returnvalue (* (`SceneComponent.GetUpVector` _staticmesh_2) -75)) "TraceTypeQuery1"))
  (if _returnvalue_2
    (bind (_bblockinghit _binitialoverlap _time _distance _location _impactpoint _normal) (`GameplayStatics.BreakHitResult` _outhit))
    (`SceneComponent.K2_SetWorldLocationAndRotation` (`self.StaticMesh`) _location (`KismetMathLibrary.MakeRotFromZX` _normal (`SceneComponent.GetForwardVector` (`self.StaticMesh`))) false false)
    (`PrimitiveComponent.SetSimulatePhysics` _staticmesh false)
    (`PrimitiveComponent.SetEnableGravity` _staticmesh false)
    (`KismetSystemLibrary.Delay` 5.0)
    (`self.K2_DestroyActor`)))

(fn `UserConstructionScript`)