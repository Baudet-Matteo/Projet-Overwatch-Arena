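; BP_C4 is a C4 explosive actor that sticks to surfaces and detonates.
; Each Tick it traces a short way along its mesh's down vector and, on a hit, snaps to the surface normal and disables physics and gravity.
; It explodes when SuperMegaChara's TriggerC4 event fires or after a short post-attach delay.
; Detonation passes the direction toward the character's camera to CallExplosion, then destroys the actor.
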(event `self.ReceiveBeginPlay`
  (bind _returnvalue (`GameplayStatics.GetActorOfClass` "/Game/Blueprints/Chara/SuperMegaChara/SuperMegaChara.SuperMegaChara_C"))
  (add `/Game/Blueprints/Chara/SuperMegaChara/SuperMegaChara.TriggerC4` _returnvalue (delegate `ExplodeC4`)))

(event `ExplodeC4`
  (bind _returnvalue (`GameplayStatics.GetActorOfClass` "/Game/Blueprints/Chara/SuperMegaChara/SuperMegaChara.SuperMegaChara_C" :!label _label))
  (`self.Explosion` (`KismetMathLibrary.Normal` (- (`SceneComponent.K2_GetComponentLocation` (`/Game/FirstPerson/Blueprints/BP_FirstPersonCharacter.FirstPersonCamera` _returnvalue)) (`SceneComponent.K2_GetComponentLocation` (`self.StaticMesh`)))))
  (`KismetSystemLibrary.PrintString` "Boom")
  (`self.K2_DestroyActor`))

(event `self.ReceiveTick`
  (params (DeltaSeconds :type "Float (single-precision)"))
  (bind _staticmesh (`self.StaticMesh`))
  (bind _staticmesh_2 (`self.StaticMesh`))
  (bind _returnvalue (`SceneComponent.K2_GetComponentLocation` _staticmesh_2))
  (bind (_outhit _returnvalue_2) (`KismetSystemLibrary.LineTraceSingle` _returnvalue (+ _returnvalue (* (`SceneComponent.GetUpVector` _staticmesh_2) -100)) "TraceTypeQuery1"))
  (if _returnvalue_2
    (bind (_bblockinghit _binitialoverlap _time _distance _location _impactpoint _normal) (`GameplayStatics.BreakHitResult` _outhit))
    (`SceneComponent.K2_SetWorldLocationAndRotation` (`self.StaticMesh`) _location (`KismetMathLibrary.MakeRotFromZX` _normal (`SceneComponent.GetForwardVector` (`self.StaticMesh`))) false false)
    (`PrimitiveComponent.SetSimulatePhysics` _staticmesh false)
    (`PrimitiveComponent.SetEnableGravity` _staticmesh false)
    (`KismetSystemLibrary.Delay` 3.0)
    (goto _label)))

(fn `UserConstructionScript`)